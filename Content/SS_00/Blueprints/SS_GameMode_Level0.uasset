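; SS_GameMode_Level0 is the Level 0 game mode that tracks enemy kills, level progression and the game's end states.
; EnemyDestroyed either triggers the HUD finish on a boss kill or counts the kill, refreshes progress and raises the level every five enemies.
; PlayerDead triggers game over.
; All feedback goes through the first player controller's SS_HUD, cast separately in each event.
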(event `self.ReceiveTick`
  (params (DeltaSeconds :type "Float (single-precision)")))

(event `PlayerDead`
  ;[1 1 1] Player Dead
  (bind _asss_hud (cast `/Game/SS_00/UI/SS_HUD` (`PlayerController.GetHUD` (`GameplayStatics.GetPlayerController` 0))))
  (`/Game/SS_00/UI/SS_HUD.GameOver` _asss_hud))

(event `EnemyDestroyed`
  (params (BossFinish :type Boolean))
  ;[1 1 1] Enemy Destroyed
  (if BossFinish
    (bind _asss_hud (cast `/Game/SS_00/UI/SS_HUD` (`PlayerController.GetHUD` (`GameplayStatics.GetPlayerController` 0))))
    (`/Game/SS_00/UI/SS_HUD.Finish` _asss_hud)
    (else
      (bind _output_get (set `self.EnemiesDestroyed` (+ (`self.EnemiesDestroyed`) 1)))
      (set `self.CountEnemiesProgress` (`self.EnemiesDestroyed`))
      (`self.UpdateProgress`)
      (if (== (mod _output_get 5) 0)
        (set `self.Level` (+ (`self.Level`) 1))
        (`self.UpdatesLevels`)))))

(event `UpdateProgress`
  ;[1 1 1] update HUD
  (bind _asss_hud (cast `/Game/SS_00/UI/SS_HUD` (`PlayerController.GetHUD` (`GameplayStatics.GetPlayerController` 0))))
  (`/Game/SS_00/UI/SS_HUD.UpdateUI` _asss_hud))

(event `UpdatesLevels`
  ;[1 1 1] Update Levels
  (bind _asss_hud (cast `/Game/SS_00/UI/SS_HUD` (`PlayerController.GetHUD` (`GameplayStatics.GetPlayerController` 0))))
  (`/Game/SS_00/UI/SS_HUD.UpdatesLevels` _asss_hud))

(fn `UserConstructionScript`)